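; Foliage group Blueprint that scatters copies of MeshToUse within a circle of Radius around its origin at construction.
; The construction script loops over NumberOfFoliageToGenerate, adding a static mesh component with a flat random offset and random yaw at unit scale.
; A square root on the random distance aims at even area coverage.
; Random draws use streams made inline from RandSeed rather than one stored stream.
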(fn ConstructionScript
  (bind _rand_seed (Variables|FoliageGeneration|GetRand%20Seed))
  (bind _randomstream (Math|Random|MakeRandomStream _rand_seed))
  (bind _returnvalue (Math|Random|RandomUnitVectorfromStream _randomstream))
  (bind (_x _y) (Math|Vector|BreakVector _returnvalue))
  (Class|KismetMathLibrary|SeedRandomStream _randomstream)
  (for _index (range 0 (Variables|FoliageGeneration|GetNumber%20of%20Foliage%20to%20Generate))
    (bind _returnvalue_2 (AddComponent|AddStaticMeshComponent false (Math|Transform|MakeTransform (* (Math|Vector|Normalize (Math|Vector|MakeVector _x _y 0.0)) (* (Math|Float|Power (Math|Random|RandomFloatinRangefromStream 0.0 1.0 _randomstream) 0.5) (Variables|FoliageGeneration|GetRadius))) (Class|KismetMathLibrary|MakeRot 0.0 (Math|Random|RandomFloatinRangefromStream 0.0 3.6e+02 _randomstream) 0.0))))
    (Components|StaticMesh|SetStaticMesh _returnvalue_2 (Variables|FoliageGeneration|GetMesh%20To%20Use))))