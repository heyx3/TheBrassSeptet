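; BP_BurningMountain is a mountain actor that can catch fire and sink with a shaking motion.
; Its three fire particle systems start inactive; once the first is active, Tick ramps the light along a power curve and scales flames linearly from the same alpha.
; While IsSinking is set, it lowers an unshaken base position and adds a pseudo-random offset made by spinning a vector with game time.
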(event EventBeginPlay
  ;[1 1 1] Set up info
  (Class|LightComponent|SetBrightness (Variables|Components|GetFire%20Light) 0.0)
  (CallFunction|DeactivateParticles)
  (Variables|SinkIntoSea|SetNon-Shaking%20Pos (Transformation|GetActorLocation)))

(event EventTick
  (params (DeltaSeconds :type Float%20%28single-precision%29))
  (bind _returnvalue (Utilities|Time|GetGameTimeinSeconds))
  (Utilities|FlowControl|Sequence
    (:then_0
      ;[1 1 1] Update light brightness
      (if (Components|Activation|IsActive (Variables|Components|GetMountain%20Fire%201))
        (Variables|FlameandLightGrowth|SetCurrent%20Intensity%20Lerp (Math|Float|Clamp(Float) (+ (* DeltaSeconds (Variables|FlameandLightGrowth|GetIntensity%20Lerp%20Increase%20Speed)) (Variables|FlameandLightGrowth|GetCurrent%20Intensity%20Lerp))))
        (Class|LightComponent|SetBrightness (Variables|Components|GetFire%20Light) (Math|Float|Lerp 0.0 (Variables|FlameandLightGrowth|GetBase%20Intensity) (Math|Float|Power (Variables|FlameandLightGrowth|GetCurrent%20Intensity%20Lerp) (Variables|FlameandLightGrowth|GetIntensity%20Lerp%20Pow))))
        (else
          (Class|LightComponent|SetBrightness (Variables|Components|GetFire%20Light) 0.0))))
    (:then_1
      ;[1 1 1] Update flame particle scale
      (CallFunction|SetFireScale (Math|Vector|Lerp(Vector) "0, 0, 0" (Variables|FlameandLightGrowth|GetFinal%20Flame%20Size) (Variables|FlameandLightGrowth|GetCurrent%20Intensity%20Lerp))))
    (:then_2
      ;[1 1 1] Sinking behavior
      (if (Variables|SinkIntoSea|GetIs%20Sinking?)
        ;;[1 1 1] Sinking downward
        (Variables|SinkIntoSea|SetNon-Shaking%20Pos (+ (Variables|SinkIntoSea|GetNon-Shaking%20Pos) (* "0, 0,-1.000000" (* DeltaSeconds (Variables|SinkIntoSea|GetSink%20Speed)))))
        (Transformation|SetActorLocation (+ (Variables|SinkIntoSea|GetNon-Shaking%20Pos) (* (Math|Vector|RotateVector (Math|Vector|MakeVector 1.0 0.0 0.0) (Class|KismetMathLibrary|MakeRot (* 5625.4 _returnvalue) (* _returnvalue 1e+03) (* _returnvalue 956432.4))) (Variables|SinkIntoSea|GetShake%20Strength))) false)))))

(fn ConstructionScript
  (Variables|FlameandLightGrowth|SetBase%20Intensity (Variables|/Script/Engine.LightComponentBase|GetIntensity (Variables|Components|GetFire%20Light)))
  (Class|LightComponent|SetBrightness (Variables|Components|GetFire%20Light) 0.0)
  (CallFunction|DeactivateParticles)
  (Variables|SinkIntoSea|SetNon-Shaking%20Pos (Transformation|GetActorLocation)))

(fn DeactivateParticles
  (Components|Activation|Deactivate (Variables|Components|GetMountain%20Fire%201))
  (Components|Activation|Deactivate (Variables|Components|GetMountain%20Fire%202))
  (Components|Activation|Deactivate (Variables|Components|GetMountain%20Fire%203)))

(fn ActivateParticles
  (Components|Activation|Activate (Variables|Components|GetMountain%20Fire%201) false)
  (Components|Activation|Activate (Variables|Components|GetMountain%20Fire%202) false)
  (Components|Activation|Activate (Variables|Components|GetMountain%20Fire%203) false))

(fn SetFireScale
  (params (New%20Scale :type Vector))
  (Effects|Components|ParticleSystem|SetVectorParameter (Variables|Components|GetMountain%20Fire%201) "Flame Scale" New%20Scale)
  (Effects|Components|ParticleSystem|SetVectorParameter (Variables|Components|GetMountain%20Fire%202) "Flame Scale" New%20Scale)
  (Effects|Components|ParticleSystem|SetVectorParameter (Variables|Components|GetMountain%20Fire%203) "Flame Scale" New%20Scale))