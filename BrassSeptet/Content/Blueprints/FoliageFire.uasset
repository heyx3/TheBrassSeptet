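; FoliageFire is a fire effect actor with a light and flame particles that starts hidden and unlit.
; Once the actor is unhidden, Tick advances a clamped 0 to 1 lerp that raises the light toward its construction-time intensity along a power curve.
; The same lerp linearly grows the particles' Flame Scale parameter from zero to the final flame size.
; Nothing in this Blueprint unhides the actor or lowers the lerp.
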(event EventBeginPlay
  ;[1 1 1] Set up light brightness and visibility
  (Class|LightComponent|SetBrightness (Variables|Default|GetFireLight) 0.0)
  (Rendering|SetActorHiddenInGame true))

(event EventTick
  (params (DeltaSeconds :type Float%20%28single-precision%29))
  (Utilities|FlowControl|Sequence
    (:then_0
      ;[1 1 1] Update light brightness
      (if (not (Variables|Rendering|GetbHidden))
        (Variables|FlameandLightGrowth|SetCurrent%20Intensity%20Lerp (Math|Float|Clamp(Float) (+ (* DeltaSeconds (Variables|FlameandLightGrowth|GetIntensity%20Lerp%20Increase%20Speed)) (Variables|FlameandLightGrowth|GetCurrent%20Intensity%20Lerp))))
        (Class|LightComponent|SetBrightness (Variables|Default|GetFireLight) (Math|Float|Lerp 0.0 (Variables|FlameandLightGrowth|GetBase%20Intensity) (Math|Float|Power (Math|Float|Clamp(Float) (+ (* DeltaSeconds (Variables|FlameandLightGrowth|GetIntensity%20Lerp%20Increase%20Speed)) (Variables|FlameandLightGrowth|GetCurrent%20Intensity%20Lerp))) (Variables|FlameandLightGrowth|GetIntensity%20Lerp%20Pow))))))
    (:then_1
      ;[1 1 1] Update flame particle scale
      (Effects|Components|ParticleSystem|SetVectorParameter (Variables|Default|GetParticles) "Flame Scale" (Math|Vector|Lerp(Vector) "0, 0, 0" (Variables|FlameandLightGrowth|GetFinal%20Flame%20Size) (Variables|FlameandLightGrowth|GetCurrent%20Intensity%20Lerp))))))

(fn ConstructionScript
  (Variables|FlameandLightGrowth|SetBase%20Intensity (Variables|/Script/Engine.LightComponentBase|GetIntensity (Variables|Default|GetFireLight))))