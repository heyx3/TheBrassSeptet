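; Angel actor that shakes in place and can emit smoke.
; Every Tick sets the smoke emitter's active state from IsEmittingSmoke.
; The shake removes the previous offset, then adds a new one scaled by ShakeStrength, so it layers on the current position without drifting.
; The offset direction is pseudo-random, made by rotating a unit vector with fast-spinning angles derived from game time.
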(event EventTick
  (params (DeltaSeconds :type Float%20%28single-precision%29))
  (bind _returnvalue (Utilities|Time|GetGameTimeinSeconds))
  ;[1 1 1] Toggle smoke emitter based on state
  (Components|Activation|SetActive (Variables|Angel|GetSmoke%20Emitter) (Variables|Angel|GetIs%20Emitting%20Smoke?) false)
  ;[1 1 1] Shake
  ;;[1 1 1] Remove shake offset from position
  (Transformation|SetActorLocation (- (.Location (Math|Transform|BreakTransform (Transformation|GetActorTransform))) (Variables|Angel|GetCurrent%20Pos%20Offset)) false)
  ;;[1 1 1] New pseudo-random shake offset
  (Variables|Angel|SetCurrent%20Pos%20Offset (* (Math|Vector|RotateVector (Math|Vector|MakeVector 1.0 0.0 0.0) (Class|KismetMathLibrary|MakeRot (* 5625.4 _returnvalue) (* _returnvalue 1e+03) (* _returnvalue 956432.4))) (Variables|Angel|GetShake%20Strength)))
  ;;[1 1 1] Add shake offset to position
  (Transformation|SetActorLocation (+ (Variables|Angel|GetCurrent%20Pos%20Offset) (.Location (Math|Transform|BreakTransform (Transformation|GetActorTransform)))) false))

(fn ConstructionScript)